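; BP_Character is a character Blueprint with a Gameplay Ability System component and a melee hit sphere.
; On BeginPlay it attaches MeleeSphere to the mesh's abilityLeftSocket and applies the GE_ManaRegen effect to itself.
; When the sphere begins overlapping another BP_Character, excluding itself, it activates MeleeParticles; this graph applies no damage and never deactivates the particles.
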(event `self.ReceiveBeginPlay`
  (`SceneComponent.K2_AttachToComponent` (`self.MeleeSphere`) (`self.Mesh`) "abilityLeftSocket" "KeepRelative" "KeepRelative" "KeepRelative" true)
  (`AbilitySystemComponent.BP_ApplyGameplayEffectToSelf` :`self` (`self.AbilitySystemComponent`) :`GameplayEffectClass` "/Game/Blueprints/Abilities/GameplayEffects/GE_ManaRegen.GE_ManaRegen_C"))

(event `self.MeleeSphere.OnComponentBeginOverlap`
  (params (OverlappedComponent :type "PrimitiveComponent Object Reference") (OtherActor :type "Actor Object Reference") (OtherComp :type "PrimitiveComponent Object Reference") (OtherBodyIndex :type Integer) (bFromSweep :type Boolean) (SweepResult :type "HitResult Structure (by ref)"))
  (bind _asbp_character (cast `/Game/Blueprints/Character/BP_Character` OtherActor))
  (if (!= _asbp_character self)
    (`ActorComponent.SetActive` (`self.MeleeParticles`) true false)))

(fn `UserConstructionScript`)