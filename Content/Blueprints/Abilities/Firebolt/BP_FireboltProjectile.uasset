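; Projectile actor for the Firebolt ability, with its lifespan derived from Range and the projectile movement's initial speed.
; On hitting anything but its instigator, the authority applies instant-damage and damage-over-time Gameplay Effects to BP_Character targets through their Ability System Component.
; It then disables collision and calls DestroyEvent, which plays explosion sound and particles at the impact point before a short delayed destroy.
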(event `self.ReceiveBeginPlay`
  (`self.SetLifeSpan` (/ (`self.Range`) (`ProjectileMovementComponent.InitialSpeed` (`self.ProjectileMovementComponent`)))))

(event `InitProjectileMovement`
  (params (Velocity :type "Vector Structure"))
  ;[1 1 1] Deprecated
  (set `MovementComponent.Velocity` Velocity (`self.ProjectileMovementComponent`)))

(event `self.SphereComponent.OnComponentHit`
  (params (HitComponent :type "PrimitiveComponent Object Reference") (OtherActor :type "Actor Object Reference") (OtherComp :type "PrimitiveComponent Object Reference") (NormalImpulse :type "Vector Structure") (Hit :type "HitResult Structure (by ref)"))
  (if (!= OtherActor (`self.GetInstigator`))
    (`/Engine/EditorBlueprintResources/ActorMacros.Switch Has Authority`
      (:`Authority`
        (bind _asbp_character (cast `/Game/Blueprints/Character/BP_Character` OtherActor)
          (:`then`
            (bind _returnvalue (`AbilitySystemBlueprintLibrary.GetAbilitySystemComponent` _asbp_character))
            (`AbilitySystemComponent.BP_ApplyGameplayEffectToSelf` :`self` _returnvalue :`GameplayEffectClass` "/Game/Blueprints/Abilities/Firebolt/GE_FireboltDamage.GE_FireboltDamage_C")
            (`AbilitySystemComponent.BP_ApplyGameplayEffectToSelf` :`self` _returnvalue :`GameplayEffectClass` "/Game/Blueprints/Abilities/Firebolt/GE_Firebolt_DoT.GE_Firebolt_DoT_C"))
          (:`CastFailed`
            _))
        (`PrimitiveComponent.SetCollisionEnabled` (`self.SphereComponent`) "NoCollision")
        (`self.DestroyEvent` (`.ImpactPoint` (`GameplayStatics.BreakHitResult` Hit)))))))

(event `DestroyEvent`
  (params (DesiredLocation :type "Vector Structure"))
  (`GameplayStatics.PlaySoundAtLocation` "/Game/StarterContent/Audio/Explosion01.Explosion01" DesiredLocation (struct) 1.0 1.0 0.0 null null null)
  (`GameplayStatics.SpawnEmitterAtLocation` "/Game/StarterContent/Particles/P_Explosion.P_Explosion" DesiredLocation)
  (`KismetSystemLibrary.Delay` 0.2)
  (`self.K2_DestroyActor`))

(fn `UserConstructionScript`)