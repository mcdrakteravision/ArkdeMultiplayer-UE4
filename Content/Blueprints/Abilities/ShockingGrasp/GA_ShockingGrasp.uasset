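; Gameplay Ability for Shocking Grasp, a melee spell cast by BP_Character.
; On activation it commits the ability and plays the AM_CastShockingGrasp montage, cancelling if the owner cast or commit fails.
; The character's MeleeSphere collision is query-only while the montage plays and is disabled when it completes, blends out or is interrupted or cancelled.
; Ending the ability also deactivates the character's MeleeParticles.
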(event `self.K2_ActivateAbility`
  (bind _asbp_character (cast `/Game/Blueprints/Character/BP_Character` (`.OwnerActor` (break `GameplayAbilityActorInfo` (`self.GetActorInfo`))))
    (:`then`
      (set `self.CharacterRef` _asbp_character)
      (bind _returnvalue (`self.K2_CommitAbility`))
      (if _returnvalue
        (`AbilityTask_PlayMontageAndWait.CreatePlayMontageAndWaitProxy` "None" "/Game/RetargetAnims/AM_CastShockingGrasp.AM_CastShockingGrasp"
          (:`then`
            (`PrimitiveComponent.SetCollisionEnabled` (`/Game/Blueprints/Character/BP_Character.MeleeSphere` (`self.CharacterRef`)) "QueryOnly"))
          (:`OnCompleted`
            (`PrimitiveComponent.SetCollisionEnabled` (`/Game/Blueprints/Character/BP_Character.MeleeSphere` (`self.CharacterRef`)) "NoCollision" :!label _label)
            (`self.K2_EndAbility`))
          (:`OnBlendOut`
            (goto _label))
          (:`OnInterrupted`
            (goto _label))
          (:`OnCancelled`
            (goto _label)))
        (else
          (`self.K2_CancelAbility` :!label _label_2))))
    (:`CastFailed`
      (goto _label_2))))

(event `self.K2_OnEndAbility`
  (params (bWasCancelled :type Boolean))
  (`ActorComponent.SetActive` (`/Game/Blueprints/Character/BP_Character.MeleeParticles` (`self.CharacterRef`)) false false))