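; Base collectable pickup that applies a gameplay effect to the character that overlaps its capsule collision.
; On authority, a BP_Character overlap disables collision and applies CollectableEffect through the character's Ability System Component.
; It then starts the respawn timer on its owning BP_ColectableSpawner and destroys itself, which only happens if that owner cast succeeds.
; On remote, any overlap destroys the actor directly, with no character check.
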(event `self.CollisionCapsuleComponent.OnComponentBeginOverlap`
  (params (OverlappedComponent :type "PrimitiveComponent Object Reference") (OtherActor :type "Actor Object Reference") (OtherComp :type "PrimitiveComponent Object Reference") (OtherBodyIndex :type Integer) (bFromSweep :type Boolean) (SweepResult :type "HitResult Structure (by ref)"))
  (`/Engine/EditorBlueprintResources/ActorMacros.Switch Has Authority`
    (:`Authority`
      (bind _asbp_character (cast `/Game/Blueprints/Character/BP_Character` OtherActor))
      (`PrimitiveComponent.SetCollisionEnabled` (`self.CollisionCapsuleComponent`) "NoCollision")
      (bind _returnvalue (`AbilitySystemBlueprintLibrary.GetAbilitySystemComponent` _asbp_character))
      (`AbilitySystemComponent.BP_ApplyGameplayEffectSpecToSelf` _returnvalue (`AbilitySystemComponent.MakeOutgoingSpec` _returnvalue (`self.CollectableEffect`) 0.0 (`AbilitySystemComponent.MakeEffectContext` _returnvalue)))
      (bind _asbp_colectable_spawner (cast `/Game/Blueprints/Core/BP_ColectableSpawner` (`self.GetOwner`)))
      (`ACM_Spawner.SetupRespawnTimer` _asbp_colectable_spawner))
    (:`Remote`
      _))
  (`self.K2_DestroyActor`))

(fn `UserConstructionScript`)