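; BP_Storm is a battle-royale style storm zone that damages characters outside its circle.
; On the server, a timeline with play rate set by ScalingTime scales StormCircle horizontally between MinScale and MaxScale.
; Leaving the circle applies the GE_StormDamage gameplay effect to an ArkdeCMCharacter through its Ability System Component, and entering removes all its stacks.
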(event `self.ReceiveBeginPlay`
  (`/Engine/EditorBlueprintResources/ActorMacros.Switch Has Authority`
    (:`Authority`
      (`TimelineComponent.SetPlayRate` (`self.StormChange`) (/ 1.0 (`self.ScalingTime`)))
      (bind (_direction _size) (`Timeline|StormChange`)
        (:`Update`
          (bind _returnvalue (`KismetMathLibrary.Lerp` (`self.MinScale`) (`self.MaxScale`) _size))
          (`SceneComponent.SetWorldScale3D` (`self.StormCircle`) (`KismetMathLibrary.MakeVector` _returnvalue _returnvalue 75.0)))))))

(event `self.StormCircle.OnComponentBeginOverlap`
  (params (OverlappedComponent :type "PrimitiveComponent Object Reference") (OtherActor :type "Actor Object Reference") (OtherComp :type "PrimitiveComponent Object Reference") (OtherBodyIndex :type Integer) (bFromSweep :type Boolean) (SweepResult :type "HitResult Structure (by ref)"))
  (`/Engine/EditorBlueprintResources/ActorMacros.Switch Has Authority`
    (:`Authority`
      (bind _asarkde_cmcharacter (cast `ArkdeCMCharacter` OtherActor))
      (bind _returnvalue (`ArkdeCMCharacter.GetAbilitySystemComponent` _asarkde_cmcharacter))
      (`/Engine/EditorBlueprintResources/StandardMacros.IsValid` _returnvalue
        (:`Is Valid`
          (`AbilitySystemComponent.RemoveActiveGameplayEffectBySourceEffect` _returnvalue "/Game/Blueprints/Abilities/Storm/GE_StormDamage.GE_StormDamage_C" null -1))))))

(event `self.StormCircle.OnComponentEndOverlap`
  (params (OverlappedComponent :type "PrimitiveComponent Object Reference") (OtherActor :type "Actor Object Reference") (OtherComp :type "PrimitiveComponent Object Reference") (OtherBodyIndex :type Integer))
  (`/Engine/EditorBlueprintResources/ActorMacros.Switch Has Authority`
    (:`Authority`
      (bind _asarkde_cmcharacter (cast `ArkdeCMCharacter` OtherActor))
      (`AbilitySystemComponent.BP_ApplyGameplayEffectToSelf` :`self` (`ArkdeCMCharacter.GetAbilitySystemComponent` _asarkde_cmcharacter) :`GameplayEffectClass` "/Game/Blueprints/Abilities/Storm/GE_StormDamage.GE_StormDamage_C"))))

(fn `UserConstructionScript`)